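; An ocean sound actor that switches between waves and underwater audio based on whether the camera is submerged.
; On BeginPlay it finds the Oceanology infinite ocean, then each Tick compares camera height to the wave solver's height there.
; Two cross-resetting DoOnce gates limit sound changes to surface crossings.
; With camera-based sound disabled, both sounds start at BeginPlay.
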(event Custom|Start%20sound
  ;[0 0 0 1 150] Sound effects
  ;;[0.07129 0 0.3333] Activate underwater sound effect
  (Audio|Components|Audio|Play (Variables|Default|GetUnderwater) 0.0)
  (Audio|Components|Audio|StopDelayed (Variables|Default|GetWaves) 0.0))

(event Custom|Stop%20sound
  ;[0 0 0 1 150] Sound effects
  ;;[0.07129 0 0.3333] Activate underwater sound effect
  (Audio|Components|Audio|StopDelayed (Variables|Default|GetUnderwater) 0.0)
  (Audio|Components|Audio|Play (Variables|Default|GetWaves) 0.0))

(event EventTick
  (params (DeltaSeconds :type Float%20%28single-precision%29))
  (bind _returnvalue (Game|GetPlayerCameraManager 0))
  (bind _returnvalue_2 (Camera|GetCameraLocation _returnvalue))
  ;[0 0 0 1 150] Sound effects
  (if (Variables|Default|GetEnable%20Camera%20Based%20Sound)
    (Utilities|IsValid (Variables|Default|GetOceanology)
      (:Is%20Valid
        (if (> (.Z (Math|Vector|BreakVector (Class|OceanologyWaveSolverComponent|GetWaveHeightatLocation (Class|OceanologyWaterParent|GetWaveSolver (Variables|Default|GetOceanology)) _returnvalue_2))) (.Z (Math|Vector|BreakVector _returnvalue_2)))
          (Utilities|FlowControl|DoOnce false :!label _label
            (:Completed
              (CallFunction|StartSound)
              (goto _label_2 Reset)))
          (else
            (Utilities|FlowControl|DoOnce false :!label _label_2
              (:Completed
                (CallFunction|StopSound)
                (goto _label Reset)))))))))

(event EventBeginPlay
  ;[0 0 0 1 150] Sound effects
  (if (Variables|Default|GetEnable%20Camera%20Based%20Sound)
    ;;[0 0 0] Get reference to Oceanology
    (bind _outactors (Actor|GetAllActorsOfClass "/Oceanology_Plugin/Design/Ocean/Blueprints/Ocean/BP_OceanologyInfiniteOcean.BP_OceanologyInfiniteOcean_C"))
    (Variables|Default|SetOceanology (Utilities|Array|Get(acopy) _outactors))
    (else
      (Audio|Components|Audio|Play (Variables|Default|GetUnderwater) 0.0)
      (Audio|Components|Audio|Play (Variables|Default|GetWaves) 0.0))))

(fn ConstructionScript)